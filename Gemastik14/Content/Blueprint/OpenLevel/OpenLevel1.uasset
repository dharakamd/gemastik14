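; OpenLevel1 is a trigger actor that shows the UI_OpenLevel1 widget when BP_Character overlaps its Box component.
; The overlap adds the widget to the viewport, plays its fade animation, pauses the game, switches to UI-only input with a visible cursor and prints a debug string.
; Unconnected leftover nodes for a FlipFlop and for removing the widget and unpausing never run.
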(event OnComponentBeginOverlap(Box)
  (params (OverlappedComponent :type Primitive%20Component%20Object%20Reference) (OtherActor :type Actor%20Object%20Reference) (OtherComp :type Primitive%20Component%20Object%20Reference) (OtherBodyIndex :type Integer) (bFromSweep :type Boolean) (SweepResult :type Hit%20Result%20Structure%20%28by%20ref%29))
  (bind _returnvalue (Game|GetPlayerController 0))
  (Utilities|Casting|CastToBP_Character OtherActor)
  (bind _returnvalue_2 (UserInterface|CreateWidget "/Game/UserInterface/UI_OpenLevel1.UI_OpenLevel1_C"))
  (UserInterface|Viewport|AddtoViewport _returnvalue_2 0)
  (UserInterface|Animation|PlayAnimation _returnvalue_2 (Variables|/Game/UserInterface/UI_OpenLevel1.UI_OpenLevel1_C|GetFadeAnimation _returnvalue_2) 0.0 1 "Forward" 1.0 false)
  (Game|SetGamePaused true)
  (Input|SetInputModeUIOnly _returnvalue 0 "DoNotLock")
  (Variables|/Script/Engine.PlayerController|SetbShowMouseCursor _returnvalue true)
  (Development|PrintString "Hello"))

(event EventBeginPlay)

(event Collision|EventActorBeginOverlap
  (params (OtherActor :type Actor%20Object%20Reference)))

(event EventTick
  (params (DeltaSeconds :type Float%20%28single-precision%29)))

(fn ConstructionScript)