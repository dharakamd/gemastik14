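; Bacteria enemy with health, an overhead health bar widget and an attack aimed at the player.
; Incoming damage applies after a short delay, updates the widget and destroys the actor at zero health.
; Despite its name, MeleeAttack halts movement, launches a BP_Projectile at the player's last position, then restores walking; the slash animation is unconnected.
; A sphere overlap shows the health bar only while the player character is inside.
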(event OnComponentBeginOverlap(Sphere)
  (params (OverlappedComponent :type Primitive%20Component%20Object%20Reference) (OtherActor :type Actor%20Object%20Reference) (OtherComp :type Primitive%20Component%20Object%20Reference) (OtherBodyIndex :type Integer) (bFromSweep :type Boolean) (SweepResult :type Hit%20Result%20Structure%20%28by%20ref%29))
  ;[1 1 1] Add Health Bar
  (Utilities|Casting|CastToBP_Character OtherActor)
  (Rendering|SetVisibility (Variables|Default|GetWidget) true false))

(event OnComponentEndOverlap(Sphere)
  (params (OverlappedComponent :type Primitive%20Component%20Object%20Reference) (OtherActor :type Actor%20Object%20Reference) (OtherComp :type Primitive%20Component%20Object%20Reference) (OtherBodyIndex :type Integer))
  ;[1 1 1] Add Health Bar
  (Utilities|Casting|CastToBP_Character OtherActor)
  (Rendering|SetVisibility (Variables|Default|GetWidget) false false))

(event EventMeleeAttack
  ;[1 1 1] Perform MeleeAttack
  (Utilities|FlowControl|Delay 2.0)
  (Pawn|Components|CharacterMovement|DisableMovement (Variables|Character|GetCharacterMovement))
  (Utilities|FlowControl|Delay 1.0)
  (bind _asbp_character (Utilities|Casting|CastToBP_Character (Game|GetPlayerCharacter 0)))
  (bind _returnvalue (Game|SpawnActorfromClass "/Game/Blueprint/Enemy/Virus/BP_Projectile.BP_Projectile_C" (Math|Transform|MakeTransform (Transformation|GetWorldLocation (Variables|Default|GetArrow1)) (Transformation|GetWorldRotation (Variables|Collision|GetCapsuleComponent)) "1,1,1") "Undefined" 0 0))
  (Physics|SetPhysicsLinearVelocity (Variables|/Game/Blueprint/Enemy/Virus/BP_Projectile.BP_Projectile_C|GetSphere _returnvalue) (* (Math|Vector|GetUnitDirection(Vector) (Transformation|GetActorLocation _returnvalue) (Class|CharacterMovementComponent|GetLastUpdateLocation (Variables|/Script/Engine.Character|GetCharacterMovement _asbp_character))) 2e+03) false "None")
  (Utilities|FlowControl|Delay 1.0)
  (Pawn|Components|CharacterMovement|SetMovementMode (Variables|Character|GetCharacterMovement) "MOVE_Walking" 0))

(event EventBeginPlay
  ;[1 1 1] Add Health Bar
  (bind _asui_enemy_1 (Utilities|Casting|CastToUI_Enemy_1 (UserInterface|GetUserWidgetObject (Variables|Default|GetWidget))))
  (bind _output_get (Variables|Default|SetHealthWidgetREF _asui_enemy_1))
  (Variables|/Game/UserInterface/UI_Enemy_1.UI_Enemy_1_C|SetMaxHealth _output_get (Variables|Default|GetMaxHealth))
  (Variables|/Game/UserInterface/UI_Enemy_1.UI_Enemy_1_C|SetCurrentHealth _output_get (Variables|Default|GetCurrentHealth)))

(event Game|Damage|EventAnyDamage
  (params (Damage :type Float%20%28single-precision%29) (DamageType :type Damage%20Type%20Object%20Reference) (InstigatedBy :type Controller%20Object%20Reference) (DamageCauser :type Actor%20Object%20Reference))
  ;[1 1 1] Receive Damage on Hit
  (Utilities|FlowControl|Delay 0.2)
  (bind _output_get (Variables|Default|SetCurrentHealth (- (Variables|Default|GetCurrentHealth) Damage)))
  (bind _output_get_2 (Variables|/Game/UserInterface/UI_Enemy_1.UI_Enemy_1_C|SetCurrentHealth (Variables|Default|GetHealthWidgetREF) _output_get))
  (if (<= _output_get_2 0.0)
    (Actor|DestroyActor)
    (Development|PrintString "Enemy Killed")
    (else
      (Development|PrintString (Utilities|String|Append "Health: " (Utilities|String|ToString(Float) _output_get_2))))))

(fn ConstructionScript)