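; BP_Character is the player character, with movement, mouse-look style camera input, sprinting, a basic attack and health.
; Sprint works only while W is held, raises walk speed and disables strafing until W is released or S is pressed.
; Attack sets a timed state flag alongside a parallel cooldown, using delays.
; Damage lowers health after a short delay and only prints the result or death message; BeginPlay adds the UI_Character widget.
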(event EventBeginPlay
  ;[1 1 1] Add UI
  (bind _returnvalue (UserInterface|CreateWidget "/Game/UserInterface/UI_Character.UI_Character_C"))
  (UserInterface|Viewport|AddtoViewport _returnvalue 0))

(event Game|Damage|EventAnyDamage
  (params (Damage :type Float%20%28single-precision%29) (DamageType :type Damage%20Type%20Object%20Reference) (InstigatedBy :type Controller%20Object%20Reference) (DamageCauser :type Actor%20Object%20Reference))
  ;[1 1 1] Receive Damage on Hit
  (Utilities|FlowControl|Delay 0.2)
  (bind _output_get (Variables|Default|SetCurrentHealth (- (Variables|Default|GetCurrentHealth) Damage)))
  (if (<= _output_get 0.0)
    (Development|PrintString "You dead")
    (else
      (Development|PrintString (Utilities|String|Append "Health: " (Utilities|String|ToString(Float) _output_get))))))

(event Input|ActionEvents|InputActionSprint
  (params (Key :type Key%20Structure :default "None"))
  ;[1 1 1] BASIC MOVEMENT
  ;;[1 1 1] Sprint
  (:Pressed
    (if (stale Input|KeyboardEvents|W _output_get)
      (Variables|Default|SetBP_Sprint true)
      (Variables|/Script/Engine.CharacterMovementComponent|SetMaxWalkSpeed (Variables|Character|GetCharacterMovement) 9e+02)
      (Variables|Default|SetDisableAD true))))

(event Input|ActionEvents|InputActionAttack
  (params (Key :type Key%20Structure :default "None"))
  ;[1 1 1] Attack 1 with Cooldown
  (:Pressed
    (if (not (Variables|Default|GetSkillCooldown?))
      (Variables|Default|SetBP_Attack true)
      (Utilities|FlowControl|Sequence
        (:then_0
          (Utilities|FlowControl|Delay 1.45)
          (Variables|Default|SetBP_Attack false))
        (:then_1
          (Variables|Default|SetSkillCooldown? true)
          (Utilities|FlowControl|Delay 3.0)
          (Variables|Default|SetSkillCooldown? false)))
      (else
        (Development|PrintString "SKILL IS ON COOLDOWN")))))

(event Input|AxisEvents|InputAxisMove_Right_Left
  (params (AxisValue :type Float%20%28single-precision%29))
  ;[1 1 1] BASIC MOVEMENT
  ;;[1 1 1] Move WASD
  (if (not (Variables|Default|GetDisableAD))
    (Pawn|Input|AddMovementInput (Transformation|GetActorRightVector) AxisValue false)))

(event Input|AxisEvents|InputAxisRotate_RightLeft
  (params (AxisValue :type Float%20%28single-precision%29))
  ;[1 1 1] BASIC MOVEMENT
  ;;[1 1 1] Rotate Camera
  (Pawn|Input|AddControllerYawInput AxisValue))

(event Input|AxisEvents|InputAxisRotate_UpDown
  (params (AxisValue :type Float%20%28single-precision%29))
  ;[1 1 1] BASIC MOVEMENT
  ;;[1 1 1] Rotate Camera
  (Pawn|Input|AddControllerPitchInput AxisValue))

(event Input|AxisEvents|InputAxisMove_ForwardBackward
  (params (AxisValue :type Float%20%28single-precision%29))
  ;[1 1 1] BASIC MOVEMENT
  ;;[1 1 1] Move WASD
  (Pawn|Input|AddMovementInput (Transformation|GetActorForwardVector) AxisValue false))

(event Input|KeyboardEvents|S
  (params (Key :type Key%20Structure :default "None"))
  ;[1 1 1] BASIC MOVEMENT
  ;;[1 1 1] Sprint
  (:Pressed
    (Variables|Default|SetBP_Sprint false)
    (Variables|/Script/Engine.CharacterMovementComponent|SetMaxWalkSpeed (Variables|Character|GetCharacterMovement) 4e+02)
    (Variables|Default|SetDisableAD false)))

(event Input|KeyboardEvents|W
  (params (Key :type Key%20Structure :default "None"))
  ;[1 1 1] BASIC MOVEMENT
  ;;[1 1 1] Sprint
  (:Pressed
    (bind _output_get (Variables|Default|SetBP_Forward true)))
  (:Released
    (Variables|Default|SetBP_Forward false)
    (Variables|Default|SetBP_Sprint false)
    (Variables|/Script/Engine.CharacterMovementComponent|SetMaxWalkSpeed (Variables|Character|GetCharacterMovement) 4e+02)
    (Variables|Default|SetDisableAD false)))

(fn ConstructionScript)