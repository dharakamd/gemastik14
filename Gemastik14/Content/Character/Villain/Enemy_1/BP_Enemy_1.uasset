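; BP_Enemy_1 is a basic villain enemy that takes damage and dies.
; On AnyDamage it waits briefly, subtracts the damage from its Health variable, and destroys itself when Health reaches zero or below.
; Debug print strings report the remaining health or the kill, and the construction script is empty.
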(event Game|Damage|EventAnyDamage
  (params (Damage :type Float%20%28single-precision%29) (DamageType :type Damage%20Type%20Object%20Reference) (InstigatedBy :type Controller%20Object%20Reference) (DamageCauser :type Actor%20Object%20Reference))
  (Utilities|FlowControl|Delay 0.2)
  (bind _output_get (Variables|Default|SetHealth (- (Variables|Default|GetHealth) Damage)))
  (if (<= _output_get 0.0)
    (Actor|DestroyActor)
    (Development|PrintString "Enemy Killed")
    (else
      (Development|PrintString (Utilities|String|Append "Health: " (Utilities|String|ToString(Float) _output_get))))))

(fn ConstructionScript)